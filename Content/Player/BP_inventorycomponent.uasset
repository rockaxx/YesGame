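; Player inventory component that holds a ten-slot item array and creates the WB_inventory widget to display it.
; HandleInput toggles the widget along with mouse cursor and input mode.
; PickUp sphere-traces at the player's feet for a BP_Item, filling the first slot that is empty or can stack it up to 64.
; It then reloads the widget and destroys the actor, relying on IsValid to skip remaining slots.
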(event EventBeginPlay
  (bind _returnvalue (UserInterface|CreateWidget "/Game/Inventory/Widgets/WB_inventory.WB_inventory_C"))
  (Variables|Default|SetInventoryWidget _returnvalue)
  (Utilities|Array|Resize (Variables|Default|GetItems) 10)
  (Default|LoadInventory (Variables|Default|GetInventoryWidget) self))

(event EventTick
  (params (DeltaSeconds :type Float%20%28single-precision%29)))

(fn HandleInput
  (bind _returnvalue (Game|GetPlayerController 0))
  (bind _returnvalue_2 (Game|GetPlayerController 0))
  (bind _inventorywidget (Variables|Default|GetInventoryWidget))
  (if (Widget|IsVisible (Variables|Default|GetInventoryWidget))
    (Widget|RemovefromParent _inventorywidget)
    (Variables|/Script/Engine.PlayerController|SetbShowMouseCursor _returnvalue false)
    (Input|SetInputModeGameOnly _returnvalue)
    (else
      (Variables|/Script/Engine.PlayerController|SetbShowMouseCursor _returnvalue_2 true)
      (Input|SetInputModeGameandUI _returnvalue_2 0 "DoNotLock" true)
      (UserInterface|Viewport|AddtoViewport _inventorywidget 0))))

(fn PickUp
  (bind _returnvalue (Game|GetPlayerCharacter 0))
  (bind _returnvalue_2 (Transformation|GetActorLocation _returnvalue))
  (bind _returnvalue_3 (- _returnvalue_2 "0, 0,65.000000"))
  (bind _outhit (Collision|SphereTraceByChannel _returnvalue_3 _returnvalue_3 1.2e+02 "TraceTypeQuery3" false 0 "None"))
  (bind _asbp_item (Utilities|Casting|CastToBP_Item (.HitActor (Collision|BreakHitResult _outhit)))
    (:then
      (for (_array_element _array_index) (Variables|Default|GetItems)
        (Utilities|IsValid _asbp_item
          (:Is%20Valid
            (if (Math|Boolean|ANDBoolean (Utilities|Enum|Equal(Enum) (.Name (Utilities|Struct|BreakS_ItemStructure _array_element)) (.Name (Utilities|Struct|BreakS_ItemStructure (Variables|/Game/Inventory/Inventory_BP/BP_Item.BP_Item_C|GetItem _asbp_item)))) (.Stackable (Utilities|Struct|BreakS_ItemStructure (Variables|/Game/Inventory/Inventory_BP/BP_Item.BP_Item_C|GetItem _asbp_item))) (<= (+ (.Quantity (Utilities|Struct|BreakS_ItemStructure _array_element)) (.Quantity (Utilities|Struct|BreakS_ItemStructure (Variables|/Game/Inventory/Inventory_BP/BP_Item.BP_Item_C|GetItem _asbp_item)))) 64))
              (Utilities|Array|SetArrayElem (Variables|Default|GetItems) _array_index (Utilities|Struct|MakeS_ItemStructure (.name (Variables|/Game/Inventory/Inventory_BP/BP_Item.BP_Item_C|GetItem _asbp_item)) (.stackable (Variables|/Game/Inventory/Inventory_BP/BP_Item.BP_Item_C|GetItem _asbp_item)) (+ (.Quantity (Utilities|Struct|BreakS_ItemStructure _array_element)) (.Quantity (Utilities|Struct|BreakS_ItemStructure (Variables|/Game/Inventory/Inventory_BP/BP_Item.BP_Item_C|GetItem _asbp_item)))) (.thumbnail (Variables|/Game/Inventory/Inventory_BP/BP_Item.BP_Item_C|GetItem _asbp_item)) (.mesh (Variables|/Game/Inventory/Inventory_BP/BP_Item.BP_Item_C|GetItem _asbp_item))))
              (Default|LoadInventory (Variables|Default|GetInventoryWidget) self :!label _label)
              (Actor|DestroyActor _asbp_item)
              (elif (== (.Quantity (Utilities|Struct|BreakS_ItemStructure _array_element)) 0)
                (Utilities|Array|SetArrayElem (Variables|Default|GetItems) _array_index (Variables|/Game/Inventory/Inventory_BP/BP_Item.BP_Item_C|GetItem _asbp_item))
                (goto _label)))))))
    (:CastFailed
      (Development|PrintString "Hello"))))